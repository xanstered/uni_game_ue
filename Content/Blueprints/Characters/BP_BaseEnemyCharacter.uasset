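; Base enemy character Blueprint that handles weapon equipping, hit reactions and death.
; BeginPlay and the AttributesComponent death event share one chain that binds Handle_Death_BP, then spawns BP_EnemyWeapon onto the mesh's weapon socket.
; GetHit calls the parent, plays a hit montage and prints current health for debugging.
; Handle_Death_BP plays the death montage, waits, then sets a lifespan to remove the actor.
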(event OnDeathDelegate(AttributesComponent)
  (EventDispatchers|AssignOnDeathDelegate (Variables|Default|GetAttributesComponent) (delegate Custom|Handle_Death_BP))
  (bind _returnvalue (Game|SpawnActorfromClass "/Game/Blueprints/Items/BP_EnemyWeapon.BP_EnemyWeapon_C" (Math|Transform|MakeTransform "0, 0, 0") "Undefined" "MultiplyWithRoot" 0 0))
  (Transformation|AttachComponentToComponent _returnvalue (Variables|Character|GetMesh) "EnemyWeaponSocket" "SnapToTarget" "SnapToTarget" "SnapToTarget" true)
  (Variables|Default|SetEnemyWeapon _returnvalue))

(event Custom|Handle_Death_BP
  (Animation|PlayAnimMontage "/Game/Assets/Animations/death/Death_AM.Death_AM" 1.0 "None")
  (Utilities|FlowControl|Delay 3.0)
  (Actor|SetLifeSpan 5.0))

(event EventBeginPlay
  (EventDispatchers|AssignOnDeathDelegate (Variables|Default|GetAttributesComponent) (delegate Custom|Handle_Death_BP))
  (bind _returnvalue (Game|SpawnActorfromClass "/Game/Blueprints/Items/BP_EnemyWeapon.BP_EnemyWeapon_C" (Math|Transform|MakeTransform "0, 0, 0") "Undefined" "MultiplyWithRoot" 0 0))
  (Transformation|AttachComponentToComponent _returnvalue (Variables|Character|GetMesh) "EnemyWeaponSocket" "SnapToTarget" "SnapToTarget" "SnapToTarget" true)
  (Variables|Default|SetEnemyWeapon _returnvalue))

(event Collision|EventActorBeginOverlap
  (params (OtherActor :type Actor%20Object%20Reference)))

(event EventTick
  (params (DeltaSeconds :type Float%20%28single-precision%29)))

(event EventGetHit
  (params (DamageAmount :type Float%20%28single-precision%29))
  (|CallParentFunction DamageAmount)
  (Animation|PlayAnimMontage "/Game/Assets/Animations/Lite_Magic_Pack/get_hit.get_hit" 1.0 "None")
  (Development|PrintString (Utilities|String|ToString(Float) (Class|AttributesComponent|GetHealth (Variables|Default|GetAttributesComponent)))))

(fn ConstructionScript)